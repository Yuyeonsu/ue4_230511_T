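; Game mode that shows the player's health bar UI, keeps a score and flags an explosion event.
; BeginPlay creates the PlayerUI widget and adds it to the viewport.
; Every Tick it counts all BP_Light2 actors in the world and sets Exploding once that count equals PassedLights.
; AddScore increments TotalScore by one.
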(event EventBeginPlay
  ;[1 1 1] 화면에 체력 바 표시
  (bind _returnvalue (UserInterface|CreateWidget "/Game/UMG/PlayerUI.PlayerUI_C"))
  (UserInterface|Viewport|AddtoViewport _returnvalue 0))

(event EventTick
  (params (DeltaSeconds :type Float%20%28single-precision%29))
  ;[1 1 1] 폭발 이벤트
  (bind _outactors (Actor|GetAllActorsOfClass "/Game/BluePrints/BP_Light2.BP_Light2_C"))
  (bind _output_get (Variables|Default|SetNumberOfLights (Utilities|Array|Length _outactors)))
  (if (== _output_get (Variables|Default|GetPassedLights))
    (Variables|Default|SetExploding true)))

(fn ConstructionScript)

(fn AddScore
  (Variables|Default|SetTotalScore (+ (Variables|Default|GetTotalScore) 1)))